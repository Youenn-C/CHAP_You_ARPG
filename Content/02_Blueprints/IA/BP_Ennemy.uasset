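; BP_Ennemy is an enemy Blueprint that tracks when the top-down player character is within its attack range.
; BeginPlay applies an overlay material to the mesh, and a Sphere overlap sets or clears IsAttacking as BP_TopDownCharacter enters or leaves.
; A random attack animation chain, gated by IsPlayingAnimation and a length-based Delay, is present but disconnected, so it never runs.
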(event OnComponentBeginOverlap(Sphere)
  (params (OverlappedComponent :type Primitive%20Component%20Object%20Reference) (OtherActor :type Actor%20Object%20Reference) (OtherComp :type Primitive%20Component%20Object%20Reference) (OtherBodyIndex :type Integer) (bFromSweep :type Boolean) (SweepResult :type Hit%20Result%20Structure%20%28by%20ref%29))
  (if (== OtherActor "/Game/02_Blueprints/BP_TopDownCharacter.BP_TopDownCharacter")
    (Variables|Default|SetIs_Attacking true)))

(event OnComponentEndOverlap(Sphere)
  (params (OverlappedComponent :type Primitive%20Component%20Object%20Reference) (OtherActor :type Actor%20Object%20Reference) (OtherComp :type Primitive%20Component%20Object%20Reference) (OtherBodyIndex :type Integer))
  (if (== OtherActor "/Game/02_Blueprints/BP_TopDownCharacter.BP_TopDownCharacter")
    (Variables|Default|SetIs_Attacking false)))

(event EventTick
  (params (DeltaSeconds :type Float%20%28single-precision%29)))

(event EventBeginPlay
  (Rendering|Material|SetOverlayMaterial (Variables|Character|GetMesh) "/Game/04_Materials/Animated_Materials/MI_Ennemy.MI_Ennemy" :!class /Script/Engine.MeshComponent))

(fn ConstructionScript)