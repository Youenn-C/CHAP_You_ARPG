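; BP_Coins is a collectible coin pickup that adds to the player's coin count.
; Its static mesh spins by a fixed local rotation every Tick, so the speed depends on frame rate.
; When the player character overlaps its sphere, it increments CoinsAmount on the player controller, refreshes the controller's PlayerUI counter and destroys itself.
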(event OnComponentBeginOverlap(Sphere)
  (params (OverlappedComponent :type Primitive%20Component%20Object%20Reference) (OtherActor :type Actor%20Object%20Reference) (OtherComp :type Primitive%20Component%20Object%20Reference) (OtherBodyIndex :type Integer) (bFromSweep :type Boolean) (SweepResult :type Hit%20Result%20Structure%20%28by%20ref%29))
  (bind _asbp_top_down_controller (CallFunction|GetPlayerController))
  (if (== OtherActor (CallFunction|GetPlayerCharacter))
    (bind _output_get (Variables|/Game/02_Blueprints/BP_TopDownController.BP_TopDownController_C|SetCoins_Amount _asbp_top_down_controller (+ (Variables|/Game/02_Blueprints/BP_TopDownController.BP_TopDownController_C|GetCoins_Amount _asbp_top_down_controller) 1)))
    (Default|UpdateCoinsAmount (Variables|/Game/02_Blueprints/BP_TopDownController.BP_TopDownController_C|GetPlayer_UI _asbp_top_down_controller) (Utilities|Text|ToText(Integer) _output_get))
    (Actor|DestroyActor)))

(event EventTick
  (params (DeltaSeconds :type Float%20%28single-precision%29))
  (Transformation|AddLocalRotation (Variables|Default|GetStaticMesh) "0.000000,0.000000,0.500000" false false))

(fn ConstructionScript)